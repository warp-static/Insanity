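; Game mode that continuously spawns asteroids around the player.
; Tick accumulates time and, about every half second, spawns a BP_Asteroid far away in a random direction from the player pawn.
; Each asteroid gets physics simulation enabled and a velocity aimed back at the player's position within a narrow random cone, so rocks fly roughly toward the player with some scatter.
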(event EventBeginPlay)

(event EventTick
  (params (DeltaSeconds :type Float%20%28single-precision%29))
  (if (>= (Variables|Default|Getlast%20asteroid) 0.5)
    (Variables|Default|Setdirection (Math|Random|RandomUnitVector))
    (bind _returnvalue (Game|SpawnActorfromClass "/Game/Blueprints/BP_Asteroid.BP_Asteroid_C" (Math|Conversions|ToTransform(Vector) (+ (* (Variables|Default|Getdirection) 100000) (Transformation|GetActorLocation (Game|Player|GetPlayerPawn 0)))) "Undefined" 0 0))
    (Physics|SetSimulatePhysics (Variables|/Game/Blueprints/BP_Asteroid.BP_Asteroid_C|GetMesh _returnvalue) true)
    (Physics|SetPhysicsLinearVelocity (Variables|/Game/Blueprints/BP_Asteroid.BP_Asteroid_C|GetMesh _returnvalue) (* (Math|Random|RandomUnitVectorinConeinDegrees (* (Variables|Default|Getdirection) -1) 5.0) 10000) true "None")
    (Variables|Default|Setlast%20asteroid 0.0)
    (else
      (Variables|Default|Setlast%20asteroid (+ (Variables|Default|Getlast%20asteroid) DeltaSeconds)))))

(fn ConstructionScript)